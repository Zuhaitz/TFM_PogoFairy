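; BP_Dummy is an enemy dummy actor that takes damage and is destroyed when its health runs out.
; On BeginPlay it assigns its Box collision to a custom trace channel object type.
; AnyDamage prints the current Health before subtracting the damage, then destroys the actor once Health reaches zero or below.
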(event EventBeginPlay
  (Collision|SetCollisionObjectType (Variables|Default|GetBox) "ECC_GameTraceChannel2"))

(event Game|Damage|EventAnyDamage
  (params (Damage :type Float%20%28single-precision%29) (DamageType :type Damage%20Type%20Object%20Reference) (InstigatedBy :type Controller%20Object%20Reference) (DamageCauser :type Actor%20Object%20Reference))
  (Development|PrintString (Utilities|String|ToString(Float) (Variables|Default|GetHealth)))
  (bind _output_get (Variables|Default|SetHealth (- (Variables|Default|GetHealth) Damage)))
  (if (<= _output_get 0.0)
    (Actor|DestroyActor)))

(fn ConstructionScript)