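; Fire spell Blueprint that deals repeated area damage to enemies inside its hitbox.
; Hitbox overlap events add and remove actors tagged Enemy in the HitEnemies list.
; A looping timer started on BeginPlay damages every listed enemy at the interval and amount set in SpellStructure.
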(event OnComponentBeginOverlap(Hitbox)
  (params (OverlappedComponent :type Primitive%20Component%20Object%20Reference) (OtherActor :type Actor%20Object%20Reference) (OtherComp :type Primitive%20Component%20Object%20Reference) (OtherBodyIndex :type Integer) (bFromSweep :type Boolean) (SweepResult :type Hit%20Result%20Structure%20%28by%20ref%29))
  (if (Actor|ActorHasTag OtherActor "Enemy")
    (Utilities|Array|AddUnique (Variables|Default|GetHitEnemies) OtherActor)))

(event OnComponentEndOverlap(Hitbox)
  (params (OverlappedComponent :type Primitive%20Component%20Object%20Reference) (OtherActor :type Actor%20Object%20Reference) (OtherComp :type Primitive%20Component%20Object%20Reference) (OtherBodyIndex :type Integer))
  (if (Actor|ActorHasTag OtherActor "Enemy")
    (Utilities|Array|RemoveItem (Variables|Default|GetHitEnemies) OtherActor)))

(event Custom|Damage%20Enemies
  (for _array_element (Variables|Default|GetHitEnemies)
    (Game|Damage|ApplyDamage _array_element (.damage (Variables|Default|GetSpellStructure)) 0 0)))

(event EventBeginPlay
  (Utilities|Time|SetTimerbyFunctionName 0 "Damage Enemies" (.delay (Variables|Default|GetSpellStructure)) true))

(fn ConstructionScript
  (|CallParentFunction))