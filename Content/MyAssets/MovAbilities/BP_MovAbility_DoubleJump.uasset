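; BP_MovAbility_DoubleJump is a movement ability that gives its owning character a double jump.
; When its action runs, it calls the parent action, then zeroes the character's vertical velocity while keeping horizontal speed.
; It then launches the character with its current velocity plus an upward JumpForce, overriding all axes so each jump has consistent height regardless of falling speed.
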(event EventMakeAction
  (|CallParentFunction)
  (CallFunction|BounceCharacter))

(fn BounceCharacter
  (bind _element (Variables|Default|GetElement))
  (CallFunction|ResetJumpVelocity)
  (Character|LaunchCharacter _element (+ (Transformation|GetVelocity _element) (Math|Vector|MakeVector 0.0 0.0 (Variables|Default|GetJumpForce))) true true))

(fn ResetJumpVelocity
  (bind _element (Variables|Default|GetElement))
  (bind _returnvalue (Transformation|GetVelocity _element))
  (bind (_x _y) (Math|Vector|BreakVector _returnvalue))
  (Variables|/Script/Engine.MovementComponent|SetVelocity (Variables|/Script/Engine.Character|GetCharacterMovement (Variables|Default|GetElement)) (Math|Vector|MakeVector _x _y 0.0)))