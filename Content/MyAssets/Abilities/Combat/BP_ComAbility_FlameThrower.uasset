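; Flamethrower combat ability that has a BP_Pogo element cast a breath spell while slowed down.
; On action start it saves the element's walk speed and rotation rate, calls SpawnBreath on the Pogo, then cuts movement speed and overrides turn rate.
; On action end it destroys the Breath actor and restores the saved movement values.
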(event EventMakeAction
  (|CallParentFunction)
  (CallFunction|CastBreath))

(event EventEndAction
  (|CallParentFunction)
  (CallFunction|ResetState))

(fn CastBreath
  (bind _element (Variables|Default|GetElement))
  (bind _element_2 (Variables|Default|GetElement))
  (bind _charactermovement (Variables|/Script/Engine.Character|GetCharacterMovement _element))
  (bind _charactermovement_2 (Variables|/Script/Engine.Character|GetCharacterMovement _element_2))
  (Variables|Default|SetWalkSpeed (Variables|/Script/Engine.CharacterMovementComponent|GetMaxWalkSpeed _charactermovement))
  (Variables|Default|SetRotationRate (Variables|/Script/Engine.CharacterMovementComponent|GetRotationRate _charactermovement))
  (bind _asbp_pogo (Utilities|Casting|CastToBP_Pogo (Variables|Default|GetElement)))
  (Default|SpawnBreath _asbp_pogo (Variables|Default|GetSpell))
  (Variables|/Script/Engine.CharacterMovementComponent|SetRotationRate _charactermovement_2 "0,50.000000, 0")
  (Variables|/Script/Engine.CharacterMovementComponent|SetMaxWalkSpeed _charactermovement_2 (/ (Variables|Default|GetWalkSpeed) 5.0)))

(fn ResetState
  (bind _element (Variables|Default|GetElement))
  (bind _charactermovement (Variables|/Script/Engine.Character|GetCharacterMovement _element))
  (Actor|DestroyActor (Variables|Default|GetBreath))
  (Variables|/Script/Engine.CharacterMovementComponent|SetRotationRate _charactermovement (Variables|Default|GetRotationRate))
  (Variables|/Script/Engine.CharacterMovementComponent|SetMaxWalkSpeed _charactermovement (Variables|Default|GetWalkSpeed)))