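; Combat ability that makes its Element repeatedly spit projectiles from the Spell class while the action is active.
; MakeAction sets a Shoot flag and starts a one-shot timer that re-arms itself after each shot, using the Spell class's default Delay.
; EndAction clears the flag, so the loop stops at the next tick of the timer.
; Animation events play the Default and End sections of the spell-maintain montage on the Element's mesh.
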(event Custom|Rock
  (if (Variables|Default|GetShoot)
    (CallFunction|SpitProjectiles)
    (Utilities|Time|SetTimerbyEvent (delegate Custom|Rock) (.delay (Utilities|GetClassDefaults (Variables|Default|GetSpell))))))

(event EventMakeAction
  (|CallParentFunction)
  (Variables|Default|SetShoot true)
  (Utilities|Time|SetTimerbyEvent (delegate Custom|Rock) (.delay (Utilities|GetClassDefaults (Variables|Default|GetSpell)))))

(event EventReproduceAnimation
  (|CallParentFunction)
  (Animation|Montage|PlayMontage (Variables|/Script/Engine.Character|GetMesh (Variables|Default|GetElement)) "/Game/MyAssets/Player/Model/Spells/M_Pogo_SpellMantain.M_Pogo_SpellMantain" 1.0 0.0 "Default"))

(event EventEndAction
  (|CallParentFunction)
  (Variables|Default|SetShoot false))

(event EventEndAnimation
  (|CallParentFunction)
  (Animation|Montage|PlayMontage (Variables|/Script/Engine.Character|GetMesh (Variables|Default|GetElement)) "/Game/MyAssets/Player/Model/Spells/M_Pogo_SpellMantain.M_Pogo_SpellMantain" 1.0 0.0 "End"))

(fn SpitProjectiles
  (Default|SpawnProjectile (Variables|Default|GetElement) (Variables|Default|GetSpell)))