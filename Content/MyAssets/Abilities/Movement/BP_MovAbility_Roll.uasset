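; Roll movement ability that puts its Element into a "ball mode" by retuning CharacterMovement while the action is active.
; On action start it caches walk speed, rotation rate and acceleration, then raises speed, overrides rotation rate and derives max acceleration from the cached walk speed, not the cached acceleration.
; On action end it restores the cached values.
; Both events call their parent first, and a debug "Hello" print remains.
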(event EventMakeAction
  (|CallParentFunction)
  (CallFunction|ChangeBallMode))

(event EventEndAction
  (|CallParentFunction)
  (CallFunction|ResetState))

(fn ChangeBallMode
  (bind _element (Variables|Default|GetElement))
  (bind _element_2 (Variables|Default|GetElement))
  (bind _charactermovement (Variables|/Script/Engine.Character|GetCharacterMovement _element))
  (bind _charactermovement_2 (Variables|/Script/Engine.Character|GetCharacterMovement _element_2))
  (Variables|Default|SetWalkSpeed (Variables|/Script/Engine.CharacterMovementComponent|GetMaxWalkSpeed _charactermovement))
  (Variables|Default|SetRotationRate (Variables|/Script/Engine.CharacterMovementComponent|GetRotationRate _charactermovement))
  (Variables|Default|SetAcceleration (Class|CharacterMovementComponent|GetMaxAcceleration _charactermovement))
  (Development|PrintString 0)
  (Variables|/Script/Engine.CharacterMovementComponent|SetRotationRate _charactermovement_2 "0,600.000000, 0")
  (Variables|/Script/Engine.CharacterMovementComponent|SetMaxWalkSpeed _charactermovement_2 (+ (Variables|Default|GetWalkSpeed) 1e+02))
  (Variables|/Script/Engine.CharacterMovementComponent|SetMaxAcceleration _charactermovement_2 (- (Variables|Default|GetWalkSpeed) 1e+02)))

(fn ResetState
  (bind _element (Variables|Default|GetElement))
  (bind _charactermovement (Variables|/Script/Engine.Character|GetCharacterMovement _element))
  (Variables|/Script/Engine.CharacterMovementComponent|SetRotationRate _charactermovement (Variables|Default|GetRotationRate))
  (Variables|/Script/Engine.CharacterMovementComponent|SetMaxWalkSpeed _charactermovement (Variables|Default|GetWalkSpeed))
  (Variables|/Script/Engine.CharacterMovementComponent|SetMaxAcceleration _charactermovement (Variables|Default|GetAcceleration)))