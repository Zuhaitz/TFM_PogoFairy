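; Movement ability that lets a character, with extra handling for BP_Pogo, glide down at a fixed fall speed.
; On action start it caches gravity scale and, if the character is falling, resets jump velocity, zeroes gravity, damps horizontal velocity and sets vertical velocity to GlideFallSpeed.
; BP_Pogo is also flagged as gliding with movement disabled.
; Ending the action restores gravity and those flags, then resets jump velocity again.
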(event EventMakeAction
  (|CallParentFunction)
  (Variables|Default|SetGravity%20Scale (Variables|/Script/Engine.CharacterMovementComponent|GetGravityScale (Variables|/Script/Engine.Character|GetCharacterMovement (Variables|Default|GetElement))))
  (CallFunction|GlideCharacter))

(event EventEndAction
  (|CallParentFunction)
  (CallFunction|ResetGlideVelocity))

(fn GlideCharacter
  (bind _element (Variables|Default|GetElement))
  (bind _charactermovement (Variables|/Script/Engine.Character|GetCharacterMovement _element))
  (if (AI|Components|NavMovement|IsFalling (Variables|/Script/Engine.Character|GetCharacterMovement (Variables|Default|GetElement)))
    (CallFunction|ResetJumpVelocity)
    (Variables|/Script/Engine.CharacterMovementComponent|SetGravityScale _charactermovement 0.0)
    (bind _asbp_pogo (Utilities|Casting|CastToBP_Pogo _element)
      (:then
        (Variables|/Game/MyAssets/Player/BP_Pogo.BP_Pogo_C|SetGliding? _asbp_pogo true)
        (Variables|/Game/MyAssets/Player/BP_Pogo.BP_Pogo_C|SetCanMove _asbp_pogo false))
      (:CastFailed
        _))
    (Variables|/Script/Engine.MovementComponent|SetVelocity _charactermovement (Math|Vector|MakeVector (/ (.x (Variables|/Script/Engine.MovementComponent|GetVelocity _charactermovement)) 6.0) (/ (.y (Variables|/Script/Engine.MovementComponent|GetVelocity _charactermovement)) 6.0) (Variables|Default|GetGlideFallSpeed)))))

(fn ResetGlideVelocity
  (bind _element (Variables|Default|GetElement))
  (Variables|/Script/Engine.CharacterMovementComponent|SetGravityScale (Variables|/Script/Engine.Character|GetCharacterMovement _element) (Variables|Default|GetGravity%20Scale))
  (bind _asbp_pogo (Utilities|Casting|CastToBP_Pogo _element)
    (:then
      (Variables|/Game/MyAssets/Player/BP_Pogo.BP_Pogo_C|SetGliding? _asbp_pogo false)
      (Variables|/Game/MyAssets/Player/BP_Pogo.BP_Pogo_C|SetCanMove _asbp_pogo true))
    (:CastFailed
      _))
  (CallFunction|ResetJumpVelocity))